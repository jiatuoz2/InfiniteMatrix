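; BP_Enemy is an enemy actor that is destroyed on contact with a projectile or the player.
; Its Cone component's begin-overlap event casts the other actor to BP_Projectiles, then to BP_Player, ignoring anything else.
; A player hit also takes one point off the player's Health; at zero it sets IsDead and calls DisplayRestart on the player.
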(event OnComponentBeginOverlap(Cone)
  (params (OverlappedComponent :type Primitive%20Component%20Object%20Reference) (OtherActor :type Actor%20Object%20Reference) (OtherComp :type Primitive%20Component%20Object%20Reference) (OtherBodyIndex :type Integer) (bFromSweep :type Boolean) (SweepResult :type Hit%20Result%20Structure%20%28by%20ref%29))
  (Utilities|Casting|CastToBP_Projectiles OtherActor
    (:then
      (Actor|DestroyActor))
    (:CastFailed
      (bind _asbp_player (Utilities|Casting|CastToBP_Player OtherActor))
      (Actor|DestroyActor)
      (bind _output_get (Variables|/Game/InfiniteMatrix/Blueprints/BP_Player.BP_Player_C|SetHealth _asbp_player (- (Variables|/Game/InfiniteMatrix/Blueprints/BP_Player.BP_Player_C|GetHealth _asbp_player) 1)))
      (if (not (Math|Conversions|ToBoolean(Integer) _output_get))
        (Variables|/Game/InfiniteMatrix/Blueprints/BP_Player.BP_Player_C|SetIsDead _asbp_player true)
        (Default|DisplayRestart _asbp_player)))))

(event EventBeginPlay)

(event Collision|EventActorBeginOverlap
  (params (OtherActor :type Actor%20Object%20Reference)))

(event EventTick
  (params (DeltaSeconds :type Float%20%28single-precision%29)))

(fn ConstructionScript)